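; Level script for Roni1_Map that builds the playfield at BeginPlay.
; It spawns Roni_BP near one corner, owned by the first player controller, and keeps a reference to it.
; Nested loops then tile a flat grid of CubeCurtain_BP actors.
; Further loops line the four edges with hidden Trace_BP actors owned by Roni, rotated on two sides to form an invisible border.
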(event `self.ReceiveBeginPlay`
  (bind _roni_bp (`self.Roni BP`))
  (bind _returnvalue (`|SpawnActorFromClass` "/Game/Blueprints/Roni_BP.Roni_BP_C" (`KismetMathLibrary.MakeTransform` (5.0 5.0 20.0)) "Undefined" "OverrideRootScale" (`GameplayStatics.GetPlayerController` 0) null))
  (set `self.Roni BP` _returnvalue)
  (`|ExecutionSequence`
    (:`then_0`
      (for _index (range 30)
        (for _index_2 (range 45)
          (`|SpawnActorFromClass` "/Game/Blueprints/CubeCurtain_BP.CubeCurtain_BP_C" (`KismetMathLibrary.MakeTransform` (`KismetMathLibrary.MakeVector` (* _index 10.0) (* _index_2 10.0) 10.0)) "Undefined" "OverrideRootScale" null null))))
    (:`then_1`
      (for _index_3 (range 28)
        (bind _returnvalue_2 (+ (* _index_3 10.0) 10.0))
        (bind _returnvalue_3 (`|SpawnActorFromClass` "/Game/Blueprints/Trace_BP.Trace_BP_C" (`KismetMathLibrary.MakeTransform` (`KismetMathLibrary.MakeVector` _returnvalue_2 4.5 20.0)) "AlwaysSpawn" "OverrideRootScale" _roni_bp null))
        (bind _returnvalue_4 (`|SpawnActorFromClass` "/Game/Blueprints/Trace_BP.Trace_BP_C" (`KismetMathLibrary.MakeTransform` (`KismetMathLibrary.MakeVector` _returnvalue_2 434.5 20.0)) "AlwaysSpawn" "OverrideRootScale" _roni_bp null))
        (`self.SetActorHiddenInGame` _returnvalue_4 true)
        (`self.SetActorHiddenInGame` _returnvalue_3 true))
      (for _index_4 (range 43)
        (bind _returnvalue_5 (+ (* _index_4 10.0) 10.0))
        (bind _returnvalue_6 (`|SpawnActorFromClass` "/Game/Blueprints/Trace_BP.Trace_BP_C" (`KismetMathLibrary.MakeTransform` (`KismetMathLibrary.MakeVector` 4.5 _returnvalue_5 20.0) (struct :`Yaw` 90.0)) "AlwaysSpawn" "OverrideRootScale" _roni_bp null))
        (bind _returnvalue_7 (`|SpawnActorFromClass` "/Game/Blueprints/Trace_BP.Trace_BP_C" (`KismetMathLibrary.MakeTransform` (`KismetMathLibrary.MakeVector` 284.5 _returnvalue_5 20.0) (struct :`Yaw` 90.0)) "AlwaysSpawn" "OverrideRootScale" _roni_bp null))
        (`self.SetActorHiddenInGame` _returnvalue_7 true)
        (`self.SetActorHiddenInGame` _returnvalue_6 true)))))

(fn `UserConstructionScript`)