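; Ghost actor that wanders a map built from CubeCurtain_BP actors, moving its Cube component on its own.
; Each Tick, IsOnTheMap box-overlaps a point one step ahead, and the Cube advances by a fixed swept offset, not scaled by delta time, while map is found.
; Otherwise, Rotation yaws it +90 degrees if that side is on the map, or -90 without checking.
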(event `self.ReceiveTick`
  (params (DeltaSeconds :type "Float (single-precision)"))
  (bind _returnvalue (`KismetMathLibrary.MakeVector` (* 10.0 1.414214)))
  (bind _isfound (`self.IsOnTheMap` (+ (+ (`SceneComponent.K2_GetComponentLocation` (`self.Cube`)) (0.0 0.0 0.0)) (`KismetMathLibrary.GreaterGreater_VectorRotator` _returnvalue (`SceneComponent.K2_GetComponentRotation` (`self.Cube`))))))
  (if _isfound
    (`SceneComponent.K2_AddLocalOffset` (`self.Cube`) _returnvalue true false)
    (else
      (`self.Rotation`))))

(fn `IsOnTheMap`
  (params (Location :type "Vector Structure"))
  (returns (IsFound :type Boolean))
  (bind _outactors (`KismetSystemLibrary.BoxOverlapActors` Location (3.0 3.0 10.0) (`|MakeArray` "ObjectTypeQuery1" :!type "EObjectTypeQuery Enum") "/Game/Blueprints/CubeCurtain_BP.CubeCurtain_BP_C"))
  (if (> (`KismetArrayLibrary.Array_Length` _outactors) 0)
    (return true)
    (else
      (return false))))

(fn `Rotation`
  (bind _cube (`self.Cube`))
  (bind _cube_2 (`self.Cube`))
  (bind _isfound (`self.IsOnTheMap` (+ (+ (`SceneComponent.K2_GetComponentLocation` (`self.Cube`)) (0.0 0.0 0.0)) (`KismetMathLibrary.GreaterGreater_VectorRotator` (`KismetMathLibrary.MakeVector` (* 10.0 1.414214)) (`KismetMathLibrary.MakeRotator` (.roll (`SceneComponent.K2_GetComponentRotation` (`self.Cube`))) (.pitch (`SceneComponent.K2_GetComponentRotation` (`self.Cube`))) (+ (.yaw (`SceneComponent.K2_GetComponentRotation` (`self.Cube`))) 90.0))))))
  (if _isfound
    (`SceneComponent.K2_SetWorldRotation` _cube_2 (`KismetMathLibrary.MakeRotator` (.roll (`SceneComponent.K2_GetComponentRotation` _cube_2)) (.pitch (`SceneComponent.K2_GetComponentRotation` _cube_2)) (+ (.yaw (`SceneComponent.K2_GetComponentRotation` _cube_2)) 90.0)) false false)
    (else
      (`SceneComponent.K2_SetWorldRotation` _cube (`KismetMathLibrary.MakeRotator` (.roll (`SceneComponent.K2_GetComponentRotation` _cube)) (.pitch (`SceneComponent.K2_GetComponentRotation` _cube)) (- (.yaw (`SceneComponent.K2_GetComponentRotation` _cube)) 90.0)) false false))))

(fn `UserConstructionScript`)