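; Clickable checker piece for a grid board game, moved one cell at a time by four directional arrows.
; Clicking the cube makes it the ChekerController's current checker, switches arrow visibility to it and spawns a particle burst.
; Visible arrows apply a swept 100-unit offset, then update the GameMode's FreeCells, refresh arrows and run the game-over check.
; Down and Left move this actor, while Up and Right move CurrentChecker; GameOver blocks all clicks.
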(event `self.DownArrow.OnClicked`
  (params (TouchedComponent :type "PrimitiveComponent Object Reference") (ButtonPressed :type "Key Structure"))
  (bind _asnrgame_mode_base_bp (cast `/Game/Blueprints/NRGameModeBaseBP` (`GameplayStatics.GetGameMode`) :!pure true))
  (bind _freecells (`/Game/Blueprints/NRGameModeBaseBP.FreeCells` _asnrgame_mode_base_bp))
  (if (not (`/Game/Blueprints/NRGameModeBaseBP.GameOver` _asnrgame_mode_base_bp))
    (bind _current_checker (`/Game/Blueprints/ChekerController.Current Checker` (stale `self.ReceiveBeginPlay` _ascheker_controller)))
    (bind _returnvalue (`self.K2_GetActorLocation` _current_checker))
    (`KismetArrayLibrary.Array_Add` _freecells _returnvalue)
    (if (not (`SceneComponent.bHiddenInGame` TouchedComponent))
      (`self.K2_AddActorWorldOffset` (-100.0 0.0 0.0) true)
      (`KismetArrayLibrary.Array_RemoveItem` _freecells _returnvalue :!label _label)
      (`/Game/Blueprints/ChekerController.Update Arrow Visability` (stale `self.ReceiveBeginPlay` _ascheker_controller) _current_checker)
      (`/Game/Blueprints/NRGameModeBaseBP.IsGameOver` _asnrgame_mode_base_bp))))

(event `self.LeftArrow.OnClicked`
  (params (TouchedComponent :type "PrimitiveComponent Object Reference") (ButtonPressed :type "Key Structure"))
  (bind _asnrgame_mode_base_bp (cast `/Game/Blueprints/NRGameModeBaseBP` (`GameplayStatics.GetGameMode`) :!pure true))
  (if (not (`/Game/Blueprints/NRGameModeBaseBP.GameOver` _asnrgame_mode_base_bp))
    (`KismetArrayLibrary.Array_Add` (`/Game/Blueprints/NRGameModeBaseBP.FreeCells` _asnrgame_mode_base_bp) (`self.K2_GetActorLocation` (`/Game/Blueprints/ChekerController.Current Checker` (stale `self.ReceiveBeginPlay` _ascheker_controller))))
    (if (not (`SceneComponent.bHiddenInGame` TouchedComponent))
      (`self.K2_AddActorWorldOffset` (0.0 -100.0 0.0) true)
      (goto _label))))

(event `self.RightArrow.OnClicked`
  (params (TouchedComponent :type "PrimitiveComponent Object Reference") (ButtonPressed :type "Key Structure"))
  (bind _asnrgame_mode_base_bp (cast `/Game/Blueprints/NRGameModeBaseBP` (`GameplayStatics.GetGameMode`) :!pure true))
  (if (not (`/Game/Blueprints/NRGameModeBaseBP.GameOver` _asnrgame_mode_base_bp))
    (bind _current_checker (`/Game/Blueprints/ChekerController.Current Checker` (stale `self.ReceiveBeginPlay` _ascheker_controller)))
    (`KismetArrayLibrary.Array_Add` (`/Game/Blueprints/NRGameModeBaseBP.FreeCells` _asnrgame_mode_base_bp) (`self.K2_GetActorLocation` _current_checker))
    (if (not (`SceneComponent.bHiddenInGame` TouchedComponent))
      (`self.K2_AddActorWorldOffset` _current_checker (0.0 100.0 0.0) true false)
      (goto _label))))

(event `self.UpArrow.OnClicked`
  (params (TouchedComponent :type "PrimitiveComponent Object Reference") (ButtonPressed :type "Key Structure"))
  (bind _asnrgame_mode_base_bp (cast `/Game/Blueprints/NRGameModeBaseBP` (`GameplayStatics.GetGameMode`) :!pure true))
  (if (not (`/Game/Blueprints/NRGameModeBaseBP.GameOver` _asnrgame_mode_base_bp))
    (bind _current_checker (`/Game/Blueprints/ChekerController.Current Checker` (stale `self.ReceiveBeginPlay` _ascheker_controller)))
    (`KismetArrayLibrary.Array_Add` (`/Game/Blueprints/NRGameModeBaseBP.FreeCells` _asnrgame_mode_base_bp) (`self.K2_GetActorLocation` _current_checker))
    (if (not (`SceneComponent.bHiddenInGame` TouchedComponent))
      (`self.K2_AddActorWorldOffset` _current_checker (100.0 0.0 0.0) true false)
      (goto _label))))

(event `self.Cube.OnClicked`
  (params (TouchedComponent :type "PrimitiveComponent Object Reference") (ButtonPressed :type "Key Structure"))
  (if (not (`/Game/Blueprints/NRGameModeBaseBP.GameOver` (cast `/Game/Blueprints/NRGameModeBaseBP` (`GameplayStatics.GetGameMode`) :!pure true)))
    (`/Game/Blueprints/ChekerController.Arrow Invisibility` (stale `self.ReceiveBeginPlay` _ascheker_controller) (`/Game/Blueprints/ChekerController.Current Checker` (stale `self.ReceiveBeginPlay` _ascheker_controller)))
    (bind _output_get (set `/Game/Blueprints/ChekerController.Current Checker` self (stale `self.ReceiveBeginPlay` _ascheker_controller)))
    (if (`KismetSystemLibrary.IsValid` _output_get)
      (`/Game/Blueprints/ChekerController.Arrow Visibility` (stale `self.ReceiveBeginPlay` _ascheker_controller) _output_get)
      (`GameplayStatics.SpawnEmitterAttached` "/Game/StarterContent/Particles/P_Explosion.P_Explosion" (`self.Cube`) "None" (0.0 0.0 50.0)))))

(event `self.ReceiveBeginPlay`
  (bind _ascheker_controller (cast `/Game/Blueprints/ChekerController` (`GameplayStatics.GetPlayerController` 0))))

(fn `UserConstructionScript`)