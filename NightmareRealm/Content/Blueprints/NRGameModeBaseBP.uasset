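; Game mode for a puzzle where tank, warplane and warship checkers must line up with their type's marker.
; SpawnCheckers shuffles positions, placing markers that set each type's target Y, plus fifteen playable checkers.
; IsGameOver sets GameOver when all fifteen match their target Y, and Restart respawns the board.
; While GameOver holds, Tick replays the end sound, calls the controller's ArrowInvisibility and adds a new game-over widget every frame.
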(event `self.ReceiveBeginPlay`
  (`GameplayStatics.PlaySound2D` "/Game/Blueprints/puzzle.puzzle" 1.0 1.0 0.0 null null)
  (`self.SpawnCheckers`))

(event `self.ReceiveTick`
  (params (DeltaSeconds :type "Float (single-precision)"))
  (bind _ascheker_controller (cast `/Game/Blueprints/ChekerController` (`GameplayStatics.GetPlayerController` 0) :!pure true))
  (if (`self.GameOver`)
    (`GameplayStatics.PlaySound2D` "/Game/Blueprints/app-29.app-29" 1.0 1.0 0.0 null null)
    (`/Game/Blueprints/ChekerController.Arrow Invisibility` _ascheker_controller (`/Game/Blueprints/ChekerController.Current Checker` _ascheker_controller))
    (bind _returnvalue (`|CreateWidget` "/Game/Blueprints/GameOverWidget.GameOverWidget_C" _ascheker_controller))
    (`UserWidget.AddToViewport` _returnvalue 0)))

(fn `IsGameOver`
  (set `self.NumberOfRightCheckers` 0)
  (for _array_element (`self.Checkers`)
    (cast `/Game/Blueprints/TankChekerBP` _array_element
      (:`then`
        (bind _y (.y (`self.K2_GetActorLocation` _array_element)))
        (if (== _y (`self.TanksY`))
          _
          (else
            (break))))
      (:`CastFailed`
        (cast `/Game/Blueprints/WarplaneChekerBP` _array_element
          (:`then`
            (if (== _y (`self.WarplanesY`))
              _
              (else
                (break))))
          (:`CastFailed`
            (cast `/Game/Blueprints/WarshipChekerBP` _array_element)
            (if (== _y (`self.WarshipsY`))
              _
              (else
                (break)))))))
    (set `self.NumberOfRightCheckers` (+ (`self.NumberOfRightCheckers`) 1)))
  (if (== (`self.NumberOfRightCheckers`) 15)
    (set `self.GameOver` true)))

(fn `Restart`
  (bind _checkers (`self.Checkers`))
  (bind _directionalcheckers (`self.DirectionalCheckers`))
  (for _array_element _checkers
    (`self.K2_DestroyActor` _array_element))
  (`KismetArrayLibrary.Array_Clear` _checkers)
  (for _array_element_2 _directionalcheckers
    (`self.K2_DestroyActor` _array_element_2))
  (`KismetArrayLibrary.Array_Clear` _directionalcheckers)
  (`self.SpawnCheckers`)
  (set `self.GameOver` false)
  (`WidgetLayoutLibrary.RemoveAllWidgets`))

(fn `SpawnCheckers`
  (bind _startcheckers (`self.StartCheckers`))
  (bind _directionalcheckers (`self.DirectionalCheckers`))
  (bind _directialcheckers (`self.DirectialCheckers`))
  (`|ExecutionSequence`
    (:`then_0`
      (`KismetArrayLibrary.Array_Shuffle` _directialcheckers)
      (for (_array_element _array_index) _directialcheckers
        (if (== _array_index 0)
          (bind _returnvalue (`KismetMathLibrary.MakeTransform` _array_element (struct) (0.85 0.85 0.1)))
          (bind _returnvalue_2 (`|SpawnActorFromClass` "/Game/Blueprints/TankChekerBP.TankChekerBP_C" _returnvalue "Undefined" "OverrideRootScale" null null))
          (bind _y (.y _array_element))
          (set `self.TanksY` _y)
          (`KismetArrayLibrary.Array_Add` _directionalcheckers _returnvalue_2)
          (elif (== _array_index 1)
            (bind _returnvalue_3 (`|SpawnActorFromClass` "/Game/Blueprints/WarplaneChekerBP.WarplaneChekerBP_C" _returnvalue "Undefined" "OverrideRootScale" null null))
            (set `self.WarplanesY` _y)
            (`KismetArrayLibrary.Array_Add` _directionalcheckers _returnvalue_3)
            (else
              (bind _returnvalue_4 (`|SpawnActorFromClass` "/Game/Blueprints/WarshipChekerBP.WarshipChekerBP_C" _returnvalue "Undefined" "OverrideRootScale" null null))
              (set `self.WarshipsY` _y)
              (`KismetArrayLibrary.Array_Add` _directionalcheckers _returnvalue_4))))))
    (:`then_1`
      (set `self.Tanks` 5)
      (set `self.Warplanes` 5)
      (set `self.Warships` 5)
      (`KismetArrayLibrary.Array_Shuffle` _startcheckers)
      (for _array_element_2 _startcheckers
        (if (> (`self.Tanks`) 0)
          (bind _returnvalue_5 (`KismetMathLibrary.MakeTransform` _array_element_2 (struct) (0.85 0.85 0.1)))
          (bind _returnvalue_6 (`|SpawnActorFromClass` "/Game/Blueprints/TankChekerBP.TankChekerBP_C" _returnvalue_5 "Undefined" "OverrideRootScale" null null))
          (set `self.Tanks` (- (`self.Tanks`) 1))
          (`KismetArrayLibrary.Array_Add` (`self.Checkers`) _returnvalue_6)
          (elif (> (`self.Warplanes`) 0)
            (bind _returnvalue_7 (`|SpawnActorFromClass` "/Game/Blueprints/WarplaneChekerBP.WarplaneChekerBP_C" _returnvalue_5 "Undefined" "OverrideRootScale" null null))
            (set `self.Warplanes` (- (`self.Warplanes`) 1))
            (`KismetArrayLibrary.Array_Add` (`self.Checkers`) _returnvalue_7)
            (elif (> (`self.Warships`) 0)
              (bind _returnvalue_8 (`|SpawnActorFromClass` "/Game/Blueprints/WarshipChekerBP.WarshipChekerBP_C" _returnvalue_5 "Undefined" "OverrideRootScale" null null))
              (set `self.Warships` (- (`self.Warships`) 1))
              (`KismetArrayLibrary.Array_Add` (`self.Checkers`) _returnvalue_8))))))))

(fn `UserConstructionScript`)