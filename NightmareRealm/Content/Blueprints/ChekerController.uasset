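; Controller for a checker board game that handles restart input and shows which directions a checker can move.
; Pressing Enter calls Restart on NRGameModeBaseBP when its GameOver flag is set.
; Move checks offset the checker's location one grid step along X and Y and look it up in the game mode's FreeCells.
; UpdateArrowVisability hides all four ChekerBP arrows, then reveals those pointing at free cells.
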(event `Key|Enter`
  (params (Key :type "Key Structure"))
  (bind _asnrgame_mode_base_bp (cast `/Game/Blueprints/NRGameModeBaseBP` (`GameplayStatics.GetGameMode`) :!pure true))
  (:`Pressed`
    (if (`/Game/Blueprints/NRGameModeBaseBP.GameOver` _asnrgame_mode_base_bp)
      (`/Game/Blueprints/NRGameModeBaseBP.Restart` _asnrgame_mode_base_bp))))

(fn `Arrow Invisibility`
  (params (Checker :type "Pawn Object Reference"))
  (bind _ascheker_bp (cast `/Game/Blueprints/ChekerBP` Checker))
  (`SceneComponent.SetHiddenInGame` (`/Game/Blueprints/ChekerBP.DownArrow` _ascheker_bp) true true)
  (`SceneComponent.SetHiddenInGame` (`/Game/Blueprints/ChekerBP.UpArrow` _ascheker_bp) true true)
  (`SceneComponent.SetHiddenInGame` (`/Game/Blueprints/ChekerBP.RightArrow` _ascheker_bp) true true)
  (`SceneComponent.SetHiddenInGame` (`/Game/Blueprints/ChekerBP.LeftArrow` _ascheker_bp) true true))

(fn `Arrow Visibility`
  (params (Checker :type "Pawn Object Reference"))
  (bind _returnvalue (`self.K2_GetActorLocation` Checker))
  (bind _ascheker_bp (cast `/Game/Blueprints/ChekerBP` Checker :!pure true))
  (`|ExecutionSequence`
    (:`then_0`
      (bind _validxy (`self.Check Valid XY` (+ _returnvalue (0.0 100.0 0.0))))
      (if _validxy
        (`SceneComponent.SetHiddenInGame` (`/Game/Blueprints/ChekerBP.RightArrow` _ascheker_bp) false true)))
    (:`then_1`
      (bind _validxy_2 (`self.Check Valid XY` (- _returnvalue (0.0 100.0 0.0))))
      (if _validxy_2
        (`SceneComponent.SetHiddenInGame` (`/Game/Blueprints/ChekerBP.LeftArrow` _ascheker_bp) false true)))
    (:`then_2`
      (bind _validxy_3 (`self.Check Valid XY` (+ _returnvalue (100.0 0.0 0.0))))
      (if _validxy_3
        (`SceneComponent.SetHiddenInGame` (`/Game/Blueprints/ChekerBP.UpArrow` _ascheker_bp) false true)))
    (:`then_3`
      (bind _validxy_4 (`self.Check Valid XY` (- _returnvalue (100.0 0.0 0.0))))
      (if _validxy_4
        (`SceneComponent.SetHiddenInGame` (`/Game/Blueprints/ChekerBP.DownArrow` _ascheker_bp) false true)))))

(fn `Check Valid XY`
  (params (XY :type "Vector Structure"))
  (returns (ValidXY :type Boolean))
  (bind _asnrgame_mode_base_bp (cast `/Game/Blueprints/NRGameModeBaseBP` (`GameplayStatics.GetGameMode`)))
  (return (`KismetArrayLibrary.Array_Contains` (`/Game/Blueprints/NRGameModeBaseBP.FreeCells` _asnrgame_mode_base_bp) XY)))

(fn `Update Arrow Visability`
  (params (Checker :type "Pawn Object Reference"))
  (`self.Arrow Invisibility` Checker)
  (`self.Arrow Visibility` Checker))

(fn `UserConstructionScript`)