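; Tetris game controller that builds a grid of Atom actors, runs falling pieces, scores cleared lines and handles game over and restart.
; Tick spawns random pieces at a random column, steps them down and fixes them when blocked, while arrow keys shift, rotate or drop.
; Pieces are rotation lists of string rows parsed into arrays, validated against the grid.
; Cells carry Occupied and Visible flags that drive actor visibility.
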(event `self.ReceiveBeginPlay`
  (bind _returnvalue (`|CreateWidget` "/Game/MyContent/Blueprints/Score.Score_C"))
  (`UserWidget.AddToViewport` _returnvalue 0)
  (`self.createMatrix`)
  (`self.UpdateBoard`)
  (`self.createShapeJ`)
  (`self.createShapeL`)
  (`self.createShapeT`)
  (`self.createShapeZ`)
  (`self.createShapeS`)
  (`self.createShapeI`)
  (`self.createShapeO`)
  (`self.GetRandomShapeWithRotation`)
  (bind _value (`self.getShape` (`self.currentShapeWithRotation`) (`self.currentRotation`)))
  (set `self.currentShape` _value))

(event `self.ReceiveTick`
  (params (DeltaSeconds :type "Float (single-precision)"))
  (bind _currentshape (`self.currentShape`))
  (if (`self.IsGameOver`)
    _
    (elif (`self.running`)
      (if (`self.needSpawnNewPiece`)
        (`self.GetRandomShapeWithRotation`)
        (bind _value (`self.getShape` (`self.currentShapeWithRotation`) (`self.currentRotation`)))
        (set `self.currentShape` _value)
        (set `self.currentXY` (`KismetMathLibrary.MakeVector2D` (`|GetArrayItem` (`|MakeArray` 0.0 1.0 2.0 3.0 4.0 5.0 6.0 7.0 8.0 9.0 :!type "Float (single-precision)") (`KismetMathLibrary.RandomIntegerInRange` 0 9))) :!label _label)
        (bind _value_2 (`self.CheckValidWithOffset` 0 0 (`self.currentShape`)))
        (if _value_2
          (`self.SpawnBlocks`)
          (if (not (`self.IsGameOver`))
            (`self.UpdateBoard`))
          (else
            (goto _label)))
        (else
          (bind _value_3 (`self.CheckValidWithOffset` 0 1 (`self.currentShape`)))
          (if _value_3
            (`KismetSystemLibrary.Delay` 0.6)
            (`self.MoveBlocks` _currentshape 0 1 _currentshape)
            (else
              (`self.FixBlocks`))))))))

(event `Key|Left`
  (params (Key :type "Key Structure"))
  (bind _currentshape (`self.currentShape`))
  (:`Pressed`
    (set `self.LeftisPressed` true)
    (if (`self.LeftisPressed`) :!label _label_2
      (bind _value (`self.CheckValidWithOffset` -1 0 (`self.currentShape`)))
      (if _value
        (`self.MoveBlocks` _currentshape -1 0 _currentshape)
        (`KismetSystemLibrary.Delay` 0.2)
        (goto _label_2))))
  (:`Released`
    (set `self.LeftisPressed` false)
    (goto _label_2)))

(event `Key|Right`
  (params (Key :type "Key Structure"))
  (bind _currentshape (`self.currentShape`))
  (:`Pressed`
    (set `self.RightisPressed` true)
    (if (`self.RightisPressed`) :!label _label_3
      (bind _value (`self.CheckValidWithOffset` 1 0 (`self.currentShape`)))
      (if _value
        (`self.MoveBlocks` _currentshape 1 0 _currentshape)
        (`KismetSystemLibrary.Delay` 0.2)
        (goto _label_3))))
  (:`Released`
    (set `self.RightisPressed` false)
    (goto _label_3)))

(event `Key|Up`
  (params (Key :type "Key Structure"))
  (bind _currentshapewithrotation (`self.currentShapeWithRotation`))
  (:`Pressed`
    (if (not (`self.IsGameOver`))
      (bind _normalizedrotation (`self.NormalizeRotation` _currentshapewithrotation (- (`self.currentRotation`) 1)))
      (bind _value (`self.getShape` _currentshapewithrotation _normalizedrotation))
      (bind _output_get (set `self.rotatedShape` _value))
      (bind _value_2 (`self.CheckValidWithOffset` 0 0 _output_get))
      (if _value_2
        (`self.MoveBlocks` (`self.currentShape`) 0 0 (`self.rotatedShape`))
        (set `self.currentShape` (`self.rotatedShape`))
        (bind _normalizedrotation_2 (`self.NormalizeRotation` (`self.currentShapeWithRotation`) (- (`self.currentRotation`) 1)))
        (set `self.currentRotation` _normalizedrotation_2)))))

(event `Key|Down`
  (params (Key :type "Key Structure"))
  (bind _currentshape (`self.currentShape`))
  (:`Pressed`
    (if (not (`self.IsGameOver`))
      (for _ (range (+ (`self.Height`) 1))
        (bind _value (`self.CheckValidWithOffset` 0 1 (`self.currentShape`)))
        (if _value
          (`self.MoveBlocks` _currentshape 0 1 _currentshape)
          (else
            (break))))
      (`self.FixBlocks`)
      (set `self.needSpawnNewPiece` true))))

(event `Key|Enter`
  (params (Key :type "Key Structure"))
  (:`Pressed`
    (if (`self.IsGameOver`)
      (for _index (range (+ (`self.Height`) 1))
        (`self.MoveUpperDown` _index))
      (set `self.IsGameOver` false)
      (set `self.full` false)
      (set `self.Score` 0)
      (set `self.running` true)
      (`WidgetLayoutLibrary.RemoveAllWidgets`)
      (bind _returnvalue (`|CreateWidget` "/Game/MyContent/Blueprints/Score.Score_C"))
      (`UserWidget.AddToViewport` _returnvalue 0)
      (`self.UpdateBoard`))))

(fn `CheckFullLine`
  (locals (full :type Boolean))
  (for (_array_element _array_index) (`self.MatrixOfAtoms`)
    (set `local.full` true)
    (for _array_element_2 (`.Line_3_761BBE124CA38BBC55C63A95BCD59742` (break `/Game/MyContent/Blueprints/LineOfAtoms` _array_element))
      (if (not (`/Game/MyContent/Blueprints/Atom.Occupied` _array_element_2))
        (set `local.full` false)))
    (if (`local.full`)
      (`self.MoveUpperDown` _array_index)
      (set `self.Score` (+ (`self.Score`) 100))
      (set `self.needSpawnNewPiece` true))))

(fn `CheckValidWithOffset`
  (params (X :type Integer) (Y :type Integer) (Shape :type "Array of /Game/MyContent/Blueprints/Line Structure"))
  (returns (value :type Boolean))
  (locals (result :type Boolean) (localX :type Integer) (localY :type Integer) (resultX :type Integer) (resultY :type Integer))
  (bind (_x _y) (`KismetMathLibrary.BreakVector2D` (`self.currentXY`)))
  (set `local.localX` X)
  (set `local.localY` Y)
  (set `local.result` true)
  (for (_array_element _array_index) Shape
    (for (_array_element_2 _array_index_2) (`.Blocks_3_3C1C28B844A9A773932A3781A8C80F9A` (break `/Game/MyContent/Blueprints/Line` _array_element))
      (set `local.resultX` (+ _array_index_2 (`KismetMathLibrary.FFloor` _x) (`local.localX`)))
      (set `local.resultY` (+ _array_index (`KismetMathLibrary.FFloor` _y) (`local.localY`)))
      (bind _value (`self.ValidXY` (`local.resultX`) (`local.resultY`)))
      (if _value
        (if (== _array_element_2 1)
          (bind _value_2 (`self.GetBlock` (`local.resultX`) (`local.resultY`)))
          (if _value_2
            (set `local.result` false)
            (return (`local.result`))))
        (else
          (set `local.result` false)
          (return (`local.result`))))))
  (return (`local.result`)))

(fn `createMatrix`
  (locals (Line :type "Array of /Game/MyContent/Blueprints/Atom Object Reference"))
  (for _index (range (+ (`self.Height`) 1))
    (`KismetArrayLibrary.Array_Clear` (`local.Line`))
    (for _index_2 (range (+ (`self.Width`) 1))
      (bind _pos (`self.GetXYPosition` (`KismetMathLibrary.Conv_IntToDouble` _index_2) (`KismetMathLibrary.Conv_IntToDouble` _index)))
      (bind _returnvalue (`|SpawnActorFromClass` "/Game/MyContent/Blueprints/Atom.Atom_C" _pos "AdjustIfPossibleButDontSpawnIfColliding" "OverrideRootScale" null _index _index_2 false false null))
      (`SceneComponent.SetVisibility` (`Actor.RootComponent` _returnvalue) true true)
      (`KismetArrayLibrary.Array_Add` (`local.Line`) _returnvalue))
    (`KismetArrayLibrary.Array_Add` (`self.MatrixOfAtoms`) (make `/Game/MyContent/Blueprints/LineOfAtoms` (`local.Line`)))))

(fn `createShapeI`
  (set `self.Shape_I` (`|MakeArray` (make `/Game/MyContent/Blueprints/Shape` (`|MakeArray` "1, 1, 1, 1")) (make `/Game/MyContent/Blueprints/Shape` (`|MakeArray` "1" "1" "1" "1")))))

(fn `createShapeJ`
  (set `self.Shape_J` (`|MakeArray` (make `/Game/MyContent/Blueprints/Shape` (`|MakeArray` "1, 1, 1" "0, 0, 1")) (make `/Game/MyContent/Blueprints/Shape` (`|MakeArray` "0, 1" "0, 1" "1, 1")) (make `/Game/MyContent/Blueprints/Shape` (`|MakeArray` "1, 0, 0" "1, 1, 1")) (make `/Game/MyContent/Blueprints/Shape` (`|MakeArray` "1, 1" "1, 0" "1, 0")))))

(fn `createShapeL`
  (set `self.Shape_L` (`|MakeArray` (make `/Game/MyContent/Blueprints/Shape` (`|MakeArray` "1, 1, 1" "1, 0, 0")) (make `/Game/MyContent/Blueprints/Shape` (`|MakeArray` "1, 1" "0, 1" "0, 1")) (make `/Game/MyContent/Blueprints/Shape` (`|MakeArray` "0, 0, 1" "1, 1, 1")) (make `/Game/MyContent/Blueprints/Shape` (`|MakeArray` "1, 0" "1, 0" "1, 1")))))

(fn `createShapeO`
  (set `self.Shape_O` (`|MakeArray` (make `/Game/MyContent/Blueprints/Shape` (`|MakeArray` "1, 1" "1, 1")))))

(fn `createShapeS`
  (set `self.Shape_S` (`|MakeArray` (make `/Game/MyContent/Blueprints/Shape` (`|MakeArray` "0, 1, 1" "1, 1, 0")) (make `/Game/MyContent/Blueprints/Shape` (`|MakeArray` "1, 0" "1, 1" "0, 1")))))

(fn `createShapeT`
  (set `self.Shape_T` (`|MakeArray` (make `/Game/MyContent/Blueprints/Shape` (`|MakeArray` "1, 1, 1" "0, 1, 0")) (make `/Game/MyContent/Blueprints/Shape` (`|MakeArray` "0, 1" "1, 1" "0, 1")) (make `/Game/MyContent/Blueprints/Shape` (`|MakeArray` "0, 1, 0" "1, 1, 1")) (make `/Game/MyContent/Blueprints/Shape` (`|MakeArray` "1, 0" "1, 1" "1, 0")))))

(fn `createShapeZ`
  (set `self.Shape_Z` (`|MakeArray` (make `/Game/MyContent/Blueprints/Shape` (`|MakeArray` "1, 1, 0" "0, 1, 1")) (make `/Game/MyContent/Blueprints/Shape` (`|MakeArray` "0, 1" "1, 1" "1, 0")))))

(fn `FixBlocks`
  (bind (_x _y) (`KismetMathLibrary.BreakVector2D` (`self.currentXY`)))
  (for (_array_element _array_index) (`self.currentShape`)
    (for (_array_element_2 _array_index_2) (`.Blocks_3_3C1C28B844A9A773932A3781A8C80F9A` (break `/Game/MyContent/Blueprints/Line` _array_element))
      (if (== _array_element_2 1)
        (bind _returnvalue (`KismetMathLibrary.FFloor` (+ _y (`KismetMathLibrary.Conv_IntToDouble` _array_index))))
        (`self.SetBlock` (`KismetMathLibrary.FFloor` (+ (`KismetMathLibrary.Conv_IntToDouble` _array_index_2) _x)) _returnvalue true true)
        (if (< _returnvalue 4)
          (if (not (`self.IsGameOver`))
            (`self.SpawnBlocks`))))))
  (`self.CheckFullLine`)
  (`self.UpdateBoard`)
  (set `self.needSpawnNewPiece` true))

(fn `GetBlock`
  (params (X :type Integer) (Y :type Integer))
  (returns (value :type Boolean))
  (return (`/Game/MyContent/Blueprints/Atom.Occupied` (`|GetArrayItem` (`.Line_3_761BBE124CA38BBC55C63A95BCD59742` (break `/Game/MyContent/Blueprints/LineOfAtoms` (`|GetArrayItem` (`self.MatrixOfAtoms`) Y))) X))))

(fn `GetRandomShapeWithRotation`
  (switch `int` (`KismetMathLibrary.RandomIntegerInRange` 0 6)
    (:`0`
      (set `self.currentShapeWithRotation` (`self.Shape_J`)))
    (:`1`
      (set `self.currentShapeWithRotation` (`self.Shape_L`)))
    (:`2`
      (set `self.currentShapeWithRotation` (`self.Shape_Z`)))
    (:`3`
      (set `self.currentShapeWithRotation` (`self.Shape_I`)))
    (:`4`
      (set `self.currentShapeWithRotation` (`self.Shape_O`)))
    (:`5`
      (set `self.currentShapeWithRotation` (`self.Shape_S`)))
    (:`6`
      (set `self.currentShapeWithRotation` (`self.Shape_T`)))))

(fn `getShape`
  (params (Shapes :type "Array of /Game/MyContent/Blueprints/Shape Structure") (rotation :type Integer))
  (returns (value :type "Array of /Game/MyContent/Blueprints/Line Structure"))
  (locals (Line :type "Array of Integer") (tempShape :type "Array of /Game/MyContent/Blueprints/Line Structure"))
  (`KismetArrayLibrary.Array_Clear` (`local.tempShape`))
  (for _array_element (`.Shape_5_F906247143A235D966E19DB61C0361BC` (break `/Game/MyContent/Blueprints/Shape` (`|GetArrayItem` Shapes rotation)))
    (for _array_element_2 (`KismetStringLibrary.ParseIntoArray` _array_element ", ")
      (`KismetArrayLibrary.Array_Add` (`local.Line`) (`KismetStringLibrary.Conv_StringToInt` _array_element_2)))
    (`KismetArrayLibrary.Array_Add` (`local.tempShape`) (make `/Game/MyContent/Blueprints/Line` (`local.Line`)))
    (`KismetArrayLibrary.Array_Clear` (`local.Line`)))
  (return (`local.tempShape`)))

(fn `GetXYPosition`
  (params (X :type "Float (double-precision)") (Y :type "Float (double-precision)"))
  (returns (pos :type "Transform Structure"))
  (return (`KismetMathLibrary.MakeTransform` (`KismetMathLibrary.MakeVector` (+ (* Y -120.0) 800.0 0.0) (+ (* X 120.0) -60.0 0.0) 180.0))))

(fn `MoveBlocks`
  (params (fromShape :type "Array of /Game/MyContent/Blueprints/Line Structure") (DeltaX :type Integer) (DeltaY :type Integer) (toShape :type "Array of /Game/MyContent/Blueprints/Line Structure"))
  (locals (index :type Integer) (localX :type "Float (double-precision)") (localY :type "Float (double-precision)"))
  (bind (_x _y) (`KismetMathLibrary.BreakVector2D` (`self.currentXY`)))
  (bind (_x_2 _y_2) (`KismetMathLibrary.BreakVector2D` (`self.currentXY`)))
  (bind (_x_3 _y_3) (`KismetMathLibrary.BreakVector2D` (`self.currentXY`)))
  (set `local.localX` (`KismetMathLibrary.Conv_IntToDouble` DeltaX))
  (set `local.localY` (`KismetMathLibrary.Conv_IntToDouble` DeltaY))
  (`|ExecutionSequence`
    (:`then_1`
      (for (_array_element _array_index) fromShape
        (for (_array_element_2 _array_index_2) (`.Blocks_3_3C1C28B844A9A773932A3781A8C80F9A` (break `/Game/MyContent/Blueprints/Line` _array_element))
          (if (== _array_element_2 1)
            (`self.SetBlock` (`KismetMathLibrary.FFloor` (+ (`KismetMathLibrary.Conv_IntToDouble` _array_index_2) _x_2)) (`KismetMathLibrary.FFloor` (+ _y_2 (`KismetMathLibrary.Conv_IntToDouble` _array_index))))))))
    (:`then_2`
      (for (_array_element_3 _array_index_3) toShape
        (for (_array_element_4 _array_index_4) (`.Blocks_3_3C1C28B844A9A773932A3781A8C80F9A` (break `/Game/MyContent/Blueprints/Line` _array_element_3))
          (if (== _array_element_4 1)
            (`self.SetBlock` (`KismetMathLibrary.FFloor` (+ (`KismetMathLibrary.Conv_IntToDouble` _array_index_4) (`local.localX`) _x_3)) (`KismetMathLibrary.FFloor` (+ _y_3 (`KismetMathLibrary.Conv_IntToDouble` _array_index_3) (`local.localY`))) false true)))))
    (:`then_3`
      (set `self.currentXY` (`KismetMathLibrary.MakeVector2D` (+ (`local.localX`) _x) (+ _y (`local.localY`)))))
    (:`then_4`
      (if (not (`self.IsGameOver`))
        (`self.UpdateBoard`)))))

(fn `MoveUpperDown`
  (params (Y :type Integer))
  (locals (line :type "Array of /Game/MyContent/Blueprints/Atom Object Reference") (index :type Integer))
  (bind _matrixofatoms (`self.MatrixOfAtoms`))
  (bind _output_get (set `local.index` Y))
  (while (> _output_get 0)
    (`KismetArrayLibrary.Array_Clear` (`local.line`))
    (for (_array_element _array_index) (`.Line_3_761BBE124CA38BBC55C63A95BCD59742` (break `/Game/MyContent/Blueprints/LineOfAtoms` (`|GetArrayItem` (`self.MatrixOfAtoms`) (`local.index`))))
      (set `/Game/MyContent/Blueprints/Atom.Occupied` (`/Game/MyContent/Blueprints/Atom.Occupied` (`|GetArrayItem` (`.Line_3_761BBE124CA38BBC55C63A95BCD59742` (break `/Game/MyContent/Blueprints/LineOfAtoms` (`|GetArrayItem` _matrixofatoms (- (`local.index`) 1)))) _array_index)) _array_element)
      (set `/Game/MyContent/Blueprints/Atom.Visible` false _array_element)
      (`KismetArrayLibrary.Array_Add` (`local.line`) _array_element))
    (`KismetArrayLibrary.Array_Set` _matrixofatoms (`local.index`) (make `/Game/MyContent/Blueprints/LineOfAtoms` (`local.line`)))
    (set `local.index` (- (`local.index`) 1))))

(fn `NormalizeRotation`
  (params (Shapes :type "Array of /Game/MyContent/Blueprints/Shape Structure") (rotation :type Integer))
  (returns (normalizedRotation :type Integer))
  (locals (r :type Integer))
  (bind _returnvalue (`KismetArrayLibrary.Array_Length` Shapes))
  (if (< rotation 0)
    (set `local.r` (+ rotation _returnvalue))
    (elif (>= rotation _returnvalue)
      (set `local.r` (- rotation _returnvalue))
      (else
        (set `local.r` rotation))))
  (return (`local.r`)))

(fn `printmatrix`
  (locals (str :type String))
  (bind _returnvalue (`KismetStringLibrary.Concat_StrStr` (`local.str`) " "))
  (for _array_element (`self.MatrixOfAtoms`)
    (for _array_element_2 (`.Line_3_761BBE124CA38BBC55C63A95BCD59742` (break `/Game/MyContent/Blueprints/LineOfAtoms` _array_element))
      (if (`/Game/MyContent/Blueprints/Atom.Occupied` _array_element_2)
        (set `local.str` (`KismetStringLibrary.Concat_StrStr` _returnvalue "1"))
        (else
          (set `local.str` (`KismetStringLibrary.Concat_StrStr` _returnvalue "0")))))
    (`KismetSystemLibrary.PrintString` (`local.str`))
    (set `local.str` ""))
  (`KismetSystemLibrary.PrintString` "================="))

(fn `SetBlock`
  (params (X :type Integer) (Y :type Integer) (fixed :type Boolean) (value :type Boolean))
  (locals (b :type "Array of Integer") (ba :type "Array of /Game/MyContent/Blueprints/Atom Object Reference") (NewLocalVar_0 :type "Array of /Game/MyContent/Blueprints/Atom Object Reference"))
  (bind _output (`|GetArrayItem` (`local.ba`) X))
  (set `local.ba` (`.Line_3_761BBE124CA38BBC55C63A95BCD59742` (break `/Game/MyContent/Blueprints/LineOfAtoms` (`|GetArrayItem` (`self.MatrixOfAtoms`) Y))))
  (if fixed
    (set `/Game/MyContent/Blueprints/Atom.Occupied` value _output)
    (else
      (set `/Game/MyContent/Blueprints/Atom.Visible` value _output)))
  (`KismetArrayLibrary.Array_Set` (`self.MatrixOfAtoms`) Y (make `/Game/MyContent/Blueprints/LineOfAtoms` (`local.ba`))))

(fn `SpawnBlocks`
  (bind _currentshape (`self.currentShape`))
  (bind (_x _y) (`KismetMathLibrary.BreakVector2D` (`self.currentXY`)))
  (if (not (`self.IsGameOver`))
    (bind _value (`self.CheckValidWithOffset` 0 0 _currentshape))
    (if _value
      (for (_array_element _array_index) _currentshape
        (for (_array_element_2 _array_index_2) (`.Blocks_3_3C1C28B844A9A773932A3781A8C80F9A` (break `/Game/MyContent/Blueprints/Line` _array_element))
          (if (== _array_element_2 1)
            (`self.SetBlock` (`KismetMathLibrary.FFloor` (+ _x (`KismetMathLibrary.Conv_IntToDouble` _array_index_2))) (`KismetMathLibrary.FFloor` (+ _y (`KismetMathLibrary.Conv_IntToDouble` _array_index))) false true)))
        (set `self.needSpawnNewPiece` false))
      (else
        (set `self.running` false)
        (`WidgetLayoutLibrary.RemoveAllWidgets`)
        (bind _returnvalue (`|CreateWidget` "/Game/MyContent/Blueprints/GameOver.GameOver_C"))
        (`UserWidget.AddToViewport` _returnvalue 0)
        (set `self.IsGameOver` true)
        (`self.FixBlocks`)))))

(fn `UpdateBoard`
  (for _array_element (`self.MatrixOfAtoms`)
    (for _array_element_2 (`.Line_3_761BBE124CA38BBC55C63A95BCD59742` (break `/Game/MyContent/Blueprints/LineOfAtoms` _array_element))
      (`SceneComponent.SetVisibility` (`/Game/MyContent/Blueprints/Atom.Scene` _array_element_2) (or (`/Game/MyContent/Blueprints/Atom.Occupied` _array_element_2) (`/Game/MyContent/Blueprints/Atom.Visible` _array_element_2)) true))))

(fn `UserConstructionScript`)

(fn `ValidXY`
  (params (X :type Integer) (Y :type Integer))
  (returns (value :type Boolean))
  (return (and (>= X 0) (<= X (`self.Width`)) (>= Y 0) (<= Y (`self.Height`)))))